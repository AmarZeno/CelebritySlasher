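; Zombie spawner actor that creates waves of ZombieCharacter_BP within its own bounds.
; SpawnZombie runs on BeginPlay and on a looping timer, growing ZombiesToSpawn each wave until it exceeds a small cap, after which nothing spawns.
; Each spawn picks random XY in the actor bounds, and GetLineTrace traces down from a fixed height to find the surface, using a hardcoded location on a miss.
; Debug strings print during spawning and tracing.
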(event EventBeginPlay
  (CallFunction|SpawnZombie)
  (Utilities|Time|SetTimerbyFunctionName 0 "SpawnZombie" 5.0 true))

(event Collision|EventActorBeginOverlap
  (params (OtherActor :type Actor%20Object%20Reference)))

(event EventTick
  (params (DeltaSeconds :type Float%20%28single-precision%29)))

(fn ConstructionScript)

(fn SpawnZombie
  (bind (_origin _boxextent) (Collision|GetActorBounds false))
  (bind _returnvalue (Math|Random|RandomPointinBoundingBox _origin _boxextent))
  (bind (_x _y) (Math|Vector|BreakVector _returnvalue))
  (if (<= (Variables|Default|GetZombiesToSpawn) 3)
    (for _index (range 1 (Variables|Default|GetZombiesToSpawn))
      (bind _newlocation (CallFunction|GetLineTrace (Math|Vector|MakeVector _x _y 3e+02)))
      (Game|SpawnActorfromClass "/Game/Blueprints/ZombieCharacter/ZombieCharacter_BP.ZombieCharacter_BP_C" (Math|Transform|MakeTransform _newlocation) "AdjustIfPossibleButAlwaysSpawn" 0 0)
      (Development|PrintString (Utilities|String|ToString(Integer) (Variables|Default|GetZombiesToSpawn))))
    (Variables|Default|SetZombiesToSpawn (+ (Variables|Default|GetZombiesToSpawn) 2))))

(fn GetLineTrace
  (params (OldPosition :type Vector))
  (bind (_x _y) (Math|Vector|BreakVector OldPosition))
  (bind _returnvalue (Math|Vector|MakeVector _x _y 0.0))
  (Development|PrintString (Utilities|String|ToString(Vector) _returnvalue))
  (bind (_outhit _returnvalue_2) (Collision|LineTraceByChannel OldPosition _returnvalue "TraceTypeQuery1" false 0 "None"))
  (if (Math|Boolean|Equal(Boolean) _returnvalue_2 false)
    (Variables|Default|SetNewLocation "110.000000,70.000000,700.000000")
    (Development|PrintString "False value")
    (else
      (Variables|Default|SetNewLocation (.Location (Collision|BreakHitResult _outhit)))))
  (return (Variables|Default|GetNewLocation)))