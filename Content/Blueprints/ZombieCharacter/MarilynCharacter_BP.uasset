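; Marilyn zombie enemy character that advances along its control rotation until flagged as hit, then explodes in a fireball and is destroyed after a delay.
; While it advances, a MoveTowardsPlayer timer periodically docks health from every Player_Pawn via ScreenFeedback, with no range check here, and silences its audio when health reaches zero.
; Cursor and touch events on its meshes toggle a MouseOver flag.
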(event OnInputTouchLeave(Mesh)
  (params (FingerIndex :type ETouchIndex%20Enum :default "Touch1") (TouchedComponent :type Primitive%20Component%20Object%20Reference))
  (Variables|Default|SetMouseOver false))

(event OnBeginCursorOver(Mesh)
  (params (TouchedComponent :type Primitive%20Component%20Object%20Reference))
  (Variables|Default|SetMouseOver true))

(event OnEndCursorOver(Mesh)
  (params (TouchedComponent :type Primitive%20Component%20Object%20Reference))
  (Variables|Default|SetMouseOver false))

(event OnInputTouchEnter(StaticMeshComponent)
  (params (FingerIndex :type ETouchIndex%20Enum :default "Touch1") (TouchedComponent :type Primitive%20Component%20Object%20Reference))
  (Variables|Default|SetMouseOver true))

(event OnInputTouchEnter(Mesh)
  (params (FingerIndex :type ETouchIndex%20Enum :default "Touch1") (TouchedComponent :type Primitive%20Component%20Object%20Reference))
  (Variables|Default|SetMouseOver true))

(event OnBeginCursorOver(StaticMeshComponent)
  (params (TouchedComponent :type Primitive%20Component%20Object%20Reference))
  (Development|PrintString "Hello")
  (Variables|Default|SetMouseOver true))

(event OnEndCursorOver(StaticMeshComponent)
  (params (TouchedComponent :type Primitive%20Component%20Object%20Reference))
  (Variables|Default|SetMouseOver false))

(event OnInputTouchLeave(StaticMeshComponent)
  (params (FingerIndex :type ETouchIndex%20Enum :default "Touch1") (TouchedComponent :type Primitive%20Component%20Object%20Reference))
  (Variables|Default|SetMouseOver false))

(event EventBeginPlay)

(event Collision|EventActorBeginOverlap
  (params (OtherActor :type Actor%20Object%20Reference)))

(event EventTick
  (params (DeltaSeconds :type Float%20%28single-precision%29))
  (bind _returnvalue (Pawn|GetControlRotation :!class /Script/Engine.Pawn))
  (bind (_roll _pitch _yaw) (Math|Rotator|BreakRotator _returnvalue))
  (if (Math|Boolean|NotEqual(Boolean) (Variables|Default|GetZDidHit) true)
    (Pawn|Input|AddMovementInput (Math|Vector|GetForwardVector (Math|Rotator|MakeRotator _roll _pitch _yaw)) (Variables|Default|GetSpeedOfMovement) false)
    (bind _returnvalue_2 (Class|MoveTowardsPlayer|GetEnemyAttackDuration (Variables|Default|GetMoveTowardsPlayer)))
    (if (>= _returnvalue_2 2.0)
      (Class|MoveTowardsPlayer|ResetStartTimer (Variables|Default|GetMoveTowardsPlayer))
      (bind _outactors (Actor|GetAllActorsOfClass "/Game/Player_Pawn.Player_Pawn_C"))
      (for _array_element _outactors
        (bind _returnvalue_3 (Class|ScreenFeedback|GetCurrentHealth (Variables|/Game/Player_Pawn.Player_Pawn_C|GetScreenFeedback _array_element)))
        (if (not (== _returnvalue_3 0.0))
          (Class|ScreenFeedback|SetCurrentHealth (Variables|/Game/Player_Pawn.Player_Pawn_C|GetScreenFeedback _array_element) (- _returnvalue_3 5.0))
          (bind _returnvalue_4 (Class|ScreenFeedback|GetCurrentHealth (Variables|/Game/Player_Pawn.Player_Pawn_C|GetScreenFeedback _array_element)))
          (Default|CallUpdateHealth _array_element _returnvalue_4)
          (bind _returnvalue_5 (Class|ScreenFeedback|GetCurrentHealth (Variables|/Game/Player_Pawn.Player_Pawn_C|GetScreenFeedback _array_element)))
          (if (== _returnvalue_5 0.0)
            (Components|Activation|Deactivate (Variables|Default|GetAudio))))))
    (else
      (Utilities|FlowControl|Delay 5.0)
      (Effects|SpawnEmitteratLocation "/Game/ExampleContent/Blueprint_Communication/Effects/P_Explosion_Fireball.P_Explosion_Fireball" (Transformation|GetWorldLocation (Variables|Character|GetMesh self)))
      (Actor|DestroyActor))))

(fn ConstructionScript)