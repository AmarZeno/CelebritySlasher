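; Zombie character Blueprint that walks forward along its control rotation every Tick at SpeedOfMovement.
; Cursor and touch enter/leave events on the Mesh and StaticMeshComponent toggle the MouseOver flag.
; Entering the StaticMeshComponent also prints debug text and traces under the cursor; if the hit actor is a SkeletalMeshActor, bones from the hit bone down switch to fully blended physics simulation.
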(event OnInputTouchLeave(Mesh)
  (params (FingerIndex :type ETouchIndex%20Enum :default "Touch1") (TouchedComponent :type Primitive%20Component%20Object%20Reference))
  (Variables|Default|SetMouseOver false))

(event OnBeginCursorOver(Mesh)
  (params (TouchedComponent :type Primitive%20Component%20Object%20Reference))
  (Variables|Default|SetMouseOver true))

(event OnEndCursorOver(Mesh)
  (params (TouchedComponent :type Primitive%20Component%20Object%20Reference))
  (Variables|Default|SetMouseOver false))

(event OnInputTouchEnter(StaticMeshComponent)
  (params (FingerIndex :type ETouchIndex%20Enum :default "Touch1") (TouchedComponent :type Primitive%20Component%20Object%20Reference))
  (bind _returnvalue (Game|GetPlayerController 0))
  (bind _hitresult (Game|Player|GetHitResultUnderCursorbyChannel _returnvalue "TraceTypeQuery1" true))
  (bind (_bblockinghit _binitialoverlap _time _location _impactpoint _normal _impactnormal _physmat _hitactor _hitcomponent _hitbonename) (Collision|BreakHitResult _hitresult))
  (Variables|Default|SetMouseOver true)
  (Development|PrintString "heyyyyyyyyy")
  (bind _asskeletal_mesh_actor (Utilities|Casting|CastToSkeletalMeshActor _hitactor))
  (Class|SkeletalMeshComponent|SetAllBodiesBelowSimulatePhysics (Variables|/Script/Engine.SkeletalMeshActor|GetSkeletalMeshComponent _asskeletal_mesh_actor) _hitbonename true true)
  (Class|SkeletalMeshComponent|SetAllBodiesBelowPhysicsBlendWeight (Variables|/Script/Engine.SkeletalMeshActor|GetSkeletalMeshComponent _asskeletal_mesh_actor) _hitbonename 1.0 false true))

(event OnInputTouchEnter(Mesh)
  (params (FingerIndex :type ETouchIndex%20Enum :default "Touch1") (TouchedComponent :type Primitive%20Component%20Object%20Reference))
  (Variables|Default|SetMouseOver true))

(event OnBeginCursorOver(StaticMeshComponent)
  (params (TouchedComponent :type Primitive%20Component%20Object%20Reference))
  (bind _returnvalue (Game|GetPlayerController 0))
  (bind _hitresult (Game|Player|GetHitResultUnderCursorbyChannel _returnvalue "TraceTypeQuery1" true))
  (bind (_bblockinghit _binitialoverlap _time _location _impactpoint _normal _impactnormal _physmat _hitactor _hitcomponent _hitbonename) (Collision|BreakHitResult _hitresult))
  (Development|PrintString "Hello")
  (Variables|Default|SetMouseOver true)
  (Development|PrintString "heyyyyyyyyy")
  (bind _asskeletal_mesh_actor (Utilities|Casting|CastToSkeletalMeshActor _hitactor))
  (Class|SkeletalMeshComponent|SetAllBodiesBelowSimulatePhysics (Variables|/Script/Engine.SkeletalMeshActor|GetSkeletalMeshComponent _asskeletal_mesh_actor) _hitbonename true true)
  (Class|SkeletalMeshComponent|SetAllBodiesBelowPhysicsBlendWeight (Variables|/Script/Engine.SkeletalMeshActor|GetSkeletalMeshComponent _asskeletal_mesh_actor) _hitbonename 1.0 false true))

(event OnEndCursorOver(StaticMeshComponent)
  (params (TouchedComponent :type Primitive%20Component%20Object%20Reference))
  (Variables|Default|SetMouseOver false))

(event OnInputTouchLeave(StaticMeshComponent)
  (params (FingerIndex :type ETouchIndex%20Enum :default "Touch1") (TouchedComponent :type Primitive%20Component%20Object%20Reference))
  (Variables|Default|SetMouseOver false))

(event EventBeginPlay)

(event Collision|EventActorBeginOverlap
  (params (OtherActor :type Actor%20Object%20Reference)))

(event EventTick
  (params (DeltaSeconds :type Float%20%28single-precision%29))
  (bind _returnvalue (Pawn|GetControlRotation :!class /Script/Engine.Pawn))
  (bind (_roll _pitch _yaw) (Math|Rotator|BreakRotator _returnvalue))
  (Pawn|Input|AddMovementInput (Math|Vector|GetForwardVector (Math|Rotator|MakeRotator _roll _pitch _yaw)) (Variables|Default|GetSpeedOfMovement) false))

(fn ConstructionScript)