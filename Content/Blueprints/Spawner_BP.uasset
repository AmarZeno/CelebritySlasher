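; Spawner actor that creates escalating waves of Zombie_BP enemies at its own location.
; BeginPlay spawns the first wave, then a looping timer calls SpawnZombie every five seconds.
; Each call spawns ZombiesToSpawn zombies with identity rotation and scale, printing the count per spawn as debug output, then raises the count by two, so waves grow without a cap.
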(event EventBeginPlay
  (CallFunction|SpawnZombie)
  (Utilities|Time|SetTimerbyFunctionName 0 "SpawnZombie" 5.0 true))

(event Collision|EventActorBeginOverlap
  (params (OtherActor :type Actor%20Object%20Reference)))

(fn ConstructionScript)

(fn SpawnZombie
  (for _index (range 1 (Variables|Default|GetZombiesToSpawn))
    (Game|SpawnActorfromClass "/Game/Blueprints/Zombie_BP.Zombie_BP_C" (Math|Transform|MakeTransform (Transformation|GetActorLocation self)) "Undefined" 0 0)
    (Development|PrintString (Utilities|String|ToString(Integer) (Variables|Default|GetZombiesToSpawn))))
  (Variables|Default|SetZombiesToSpawn (+ (Variables|Default|GetZombiesToSpawn) 2)))