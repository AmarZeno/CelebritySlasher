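; Default pawn that reads touch swipes to destroy zombies and shows the mouse cursor on play.
; Finger1 press records the start location and opens a Tick gate, which release closes.
; Once movement reaches SwipeThreshold, StartLoc jumps far off-screen to latch the swipe, so each tick destroys any Zombie_BP flagged MouseOver.
; Release prints TAP if StartLoc still matches PriorLoc, meaning no swipe registered.
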(event Collision|EventActorBeginOverlap
  (params (OtherActor :type Actor%20Object%20Reference)))

(event EventTick
  (params (DeltaSeconds :type Float%20%28single-precision%29))
  (bind _returnvalue (Game|GetPlayerController 0))
  (bind (_locationx _locationy) (Class|PlayerController|GetInputTouchState _returnvalue "Touch1"))
  (bind _returnvalue_2 (Math|Vector2D|MakeVector2D _locationx _locationy))
  (Utilities|FlowControl|Gate true
    (:Exit
      (if (>= (Math|Vector2D|Vector2DLength (- _returnvalue_2 (stale Input|ActionEvents|InputActionFinger1 _output_get))) (Variables|Default|GetSwipeThreshold))
        (Variables|Default|SetStartLoc "(X=100000.000000,Y=1000000.000000)")
        (bind _outactors (Actor|GetAllActorsOfClass "/Game/Blueprints/Zombie_BP.Zombie_BP_C"))
        (for _array_element _outactors
          (if (Variables|/Game/Blueprints/Zombie_BP.Zombie_BP_C|GetMouseOver _array_element)
            (Development|PrintString "Collided")
            (Actor|DestroyActor _array_element)
            (Variables|Default|SetPriorLoc _returnvalue_2)))))))

(event EventBeginPlay
  (Variables|/Script/Engine.PlayerController|SetbShowMouseCursor (Game|GetPlayerController 0) true))

(event Input|ActionEvents|InputActionFinger1
  (params (Key :type Key%20Structure :default "AnyKey"))
  (bind _returnvalue (Game|GetPlayerController 0))
  (bind (_locationx _locationy) (Class|PlayerController|GetInputTouchState _returnvalue "Touch1"))
  (bind _returnvalue_2 (Math|Vector2D|MakeVector2D _locationx _locationy))
  (:Pressed
    (bind _output_get (Variables|Default|SetStartLoc _returnvalue_2))
    (Variables|Default|SetPriorLoc _output_get)
    (Utilities|FlowControl|Gate true) ; enters at Open
  )
  (:Released
    (Utilities|FlowControl|Sequence
      (:then_0
        (Utilities|FlowControl|Gate true) ; enters at Close
      )
      (:then_1
        (if (Math|Vector|Equal(Vector) (Variables|Default|GetStartLoc) (Variables|Default|GetPriorLoc) 0.0001)
          (Development|PrintString "TAP"))))))

(fn ConstructionScript)